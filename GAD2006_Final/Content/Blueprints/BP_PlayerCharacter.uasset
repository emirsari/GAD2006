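; Player character Blueprint that initializes health, maximum health, walking and running speeds, and a healing rate on BeginPlay.
; A ChangeCharacterColor event stores two character materials, but the customization widget binding and mesh material assignment meant to use it are disconnected.
; HUD creation, alternate stat values and a test switch are also left as unreachable leftovers, several marked discarded or test.
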(event `ChangeCharacterColor`
  (params (NewColor_0 :type "MaterialInstance Object Reference") (NewColor_1 :type "MaterialInstance Object Reference"))
  ;[0 0 0] Discarded(characterCustomization)
  (set `self.CharMat_0` NewColor_0)
  (set `self.CharMat_1` NewColor_1))

(event `self.ReceiveBeginPlay`
  (`self.setHealth` 100.0)
  (set `self.MaxHealth` 100.0)
  (set `self.WalkingSpeed` 250.0)
  (set `self.RunningSpeed` 600.0)
  (set `self.HealingRate` 0.5))

(fn `UserConstructionScript`
  ;[0 0 0] Discarded
)