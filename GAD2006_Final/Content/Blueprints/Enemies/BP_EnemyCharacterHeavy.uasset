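; BP_EnemyCharacterHeavy is the heavy enemy character, tuned with its own health, walking speed and a zero healing rate.
; BeginPlay applies these stats, setting current and maximum health to the same value.
; Every Tick, UpdateEnemyHealthBar casts the HealthBarWidget's user widget to WBP_EnemyHealthBar and copies current health into its DisplayHealth.
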(event `self.ReceiveBeginPlay`
  (`self.setHealth` 125.0)
  (set `self.MaxHealth` 125.0)
  (set `self.HealingRate` 0.0)
  (set `self.WalkingSpeed` 150.0))

(event `self.ReceiveTick`
  (params (DeltaSeconds :type "Float (single-precision)"))
  (`self.UpdateEnemyHealthBar`))

(fn `UpdateEnemyHealthBar`
  (bind _aswbp_enemy_health_bar (cast `/Game/Blueprints/UI/WBP_EnemyHealthBar` (`WidgetComponent.GetUserWidgetObject` (`self.HealthBarWidget`))))
  (set `/Game/Blueprints/UI/WBP_EnemyHealthBar.DisplayHealth` (`self.getHealth`) _aswbp_enemy_health_bar))

(fn `UserConstructionScript`)