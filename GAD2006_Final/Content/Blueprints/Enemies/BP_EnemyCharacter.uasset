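; Enemy character Blueprint that tracks its health and shows it on an attached health bar widget.
; BeginPlay sets starting and maximum health and a zero healing rate.
; Every Tick, UpdateEnemyHealthBar casts the HealthBarWidget component's user widget to WBP_EnemyHealthBar and copies current health into its DisplayHealth.
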(event `self.ReceiveBeginPlay`
  (`self.setHealth` 100.0)
  (set `self.MaxHealth` 100.0)
  (set `self.HealingRate` 0.0))

(event `self.ReceiveTick`
  (params (DeltaSeconds :type "Float (single-precision)"))
  (`self.UpdateEnemyHealthBar`))

(fn `UpdateEnemyHealthBar`
  (bind _aswbp_enemy_health_bar (cast `/Game/Blueprints/UI/WBP_EnemyHealthBar` (`WidgetComponent.GetUserWidgetObject` (`self.HealthBarWidget`))))
  (set `/Game/Blueprints/UI/WBP_EnemyHealthBar.DisplayHealth` (`self.getHealth`) _aswbp_enemy_health_bar))

(fn `UserConstructionScript`)