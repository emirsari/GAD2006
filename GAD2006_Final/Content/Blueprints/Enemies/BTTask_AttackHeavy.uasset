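; Behavior tree task that makes a heavy enemy attack the player character when both are alive.
; It triggers the enemy's LightAttackPressed, then immediately subtracts fixed health from the player and succeeds, or fails without damage if the player is blocking.
; There is no range or hit check, and the task never calls FinishExecute when the cast fails or either character is dead.
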(event `self.ReceiveExecuteAI`
  (params (OwnerController :type "AIController Object Reference") (ControlledPawn :type "Pawn Object Reference"))
  (bind _asbp_player_character (cast `/Game/Blueprints/BP_PlayerCharacter` (`GameplayStatics.GetPlayerCharacter` 0) :!pure true))
  (bind _asbp_enemy_character_heavy (cast `/Game/Blueprints/Enemies/BP_EnemyCharacterHeavy` ControlledPawn))
  (if (`BaseCharacter.bDead` _asbp_enemy_character_heavy)
    _
    (elif (not (`BaseCharacter.bDead` _asbp_player_character))
      (`PlayerCharacter.LightAttackPressed` _asbp_enemy_character_heavy)
      (if (`PlayerCharacter.bBlocking` _asbp_player_character)
        (`self.FinishExecute` false)
        (else
          (`BaseCharacter.setHealth` _asbp_player_character (- (`BaseCharacter.getHealth` _asbp_player_character) 15.0))
          (`self.FinishExecute` true))))))